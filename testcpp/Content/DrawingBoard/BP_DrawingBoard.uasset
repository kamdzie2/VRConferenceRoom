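; BP_DrawingBoard is an unfinished drawing board meant to paint brush strokes onto the RT_DrawingBoard render target.
; ConvertWorldToUV maps a world location through the mesh's relative transform, divides by bounding-box size and clamps to 0–1.
; DrawOnBoard is empty: its dynamic M_brush material, color, size and render-target draw nodes are disconnected and never run.
; Its UVCoordinates input is unused, and the construction script is empty.
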(fn ConstructionScript)

(fn DrawonBoard
  (params (UVCoordinates :type Vector%202D%20Structure) (Color :type Linear%20Color%20Structure)))

(fn ConvertWorldtoUV
  (params (World%20Location :type Vector))
  (bind _staticmeshcomponent (Variables|Debug|GetStaticMeshComponent))
  (bind _staticmeshcomponent_2 (Variables|Debug|GetStaticMeshComponent))
  (bind _returnvalue (Transformation|GetRelativeTransform _staticmeshcomponent_2))
  (bind _staticmesh (Variables|/Script/Engine.StaticMeshComponent|GetStaticMesh _staticmeshcomponent))
  (bind _returnvalue_2 (StaticMesh|GetBoundingBox _staticmesh))
  (bind _returnvalue_3 (Math|Transform|InverseTransformLocation _returnvalue World%20Location))
  (bind (_min _max) (Utilities|Struct|BreakBox _returnvalue_2))
  (bind (_x _y) (Math|Vector|BreakVector _returnvalue_3))
  (bind _returnvalue_4 (- _max _min))
  (bind (_x_2 _y_2) (Math|Vector|BreakVector _returnvalue_4))
  (return (Math|Vector2D|MakeVector2D (Math|Float|Clamp(Float) (/ _x _x_2)) (Math|Float|Clamp(Float) (/ _y _y_2)))))