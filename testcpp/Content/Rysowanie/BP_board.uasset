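; BP_board is an unfinished drawing board Blueprint with a Plane mesh and a render target, RT_board.
; BeginPlay applies a dynamic instance of M_board to the Plane, but storing it in DynamicBrushMat is unwired.
; DrawAtPoint does nothing yet: its nodes converting a hit location to normalized, clamped plane coordinates are unused, and the draw of DynamicBrushMat into RT_board never runs.
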(event EventBeginPlay
  (bind _returnvalue (Rendering|Material|CreateDynamicMaterialInstance "/Game/Rysowanie/M_board.M_board" "None" "None" :!class /Script/Engine.KismetMaterialLibrary))
  (Rendering|Material|SetMaterial (Variables|Default|GetPlane) 0 _returnvalue))

(fn ConstructionScript)

(fn DrawatPoint
  (params (HitLocation :type Vector)))